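; Enemy Blueprint that wanders randomly and chases the player's Muh_Character when it sees it.
; While CanSeeEnemy is false, Tick waits a random few seconds, then moves to a random reachable point nearby.
; Pawn Sensing sightings set the flag and move toward the seen character.
; A retriggerable delay clears the flag shortly after sightings stop, returning it to patrol.
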(event OnSeePawn(PawnSensing)
  (params (Pawn :type Pawn%20Object%20Reference))
  ;[1 1 1] Enemy Tracking AI
  (bind _asmuh_character (Utilities|Casting|CastToMuh_Character Pawn))
  (Utilities|FlowControl|Sequence
    (:then_0
      (Variables|Default|SetCanSeeEnemy true)
      (AI|AIMoveTo self "0, 0, 0" _asmuh_character 1e+01 false))
    (:then_1
      (Utilities|FlowControl|RetriggerableDelay 0.5)
      (Variables|Default|SetCanSeeEnemy false))))

(event EventBeginPlay)

(event Collision|EventActorBeginOverlap
  (params (OtherActor :type Actor%20Object%20Reference)))

(event EventTick
  (params (DeltaSeconds :type Float%20%28single-precision%29))
  ;[1 1 1] Enemy Patrol AI
  (if (not (Variables|Default|GetCanSeeEnemy))
    (Utilities|FlowControl|Delay (Math|Random|RandomFloatinRange 1.0 3.0))
    (AI|AIMoveTo self (.RandomLocation (AI|Navigation|GetRandomReachablePointinRadius (Transformation|GetActorLocation) 1e+03 0 0)) 0 5.0 false)))

(fn ConstructionScript)